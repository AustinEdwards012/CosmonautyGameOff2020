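; BP_Werewolf is a boss that throws projectiles at the player, takes damage from enemy characters and opens the ending cutscene when defeated.
; An attack loop, gated by player visibility and hit state, spawns randomly offset BP_GunProjectile throws between timed delays, while a repeating aim macro yaws the capsule toward the player.
; Enemies overlapping the hitbox are killed and cost one health; DoOnce blocks further hits during stagger, after which attacking restarts.
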(event `self.ReceiveBeginPlay`
  ;[1 1 1] Event Begin Play
  (bind _asbp_player_character (cast `/Game/Blueprints/Player/BP_PlayerCharacter` (`GameplayStatics.GetPlayerCharacter` 0)))
  (set `self.Player` _asbp_player_character)
  (`self.Attack`))

(event `self.Hitbox.OnComponentBeginOverlap`
  (params (OverlappedComponent :type "PrimitiveComponent Object Reference") (OtherActor :type "Actor Object Reference") (OtherComp :type "PrimitiveComponent Object Reference") (OtherBodyIndex :type Integer) (bFromSweep :type Boolean) (SweepResult :type "HitResult Structure (by ref)"))
  ;[1 1 1] Take Hit
  (bind _asbp_enemy_character (cast `/Game/Blueprints/Enemy/BP_EnemyCharacter` OtherActor))
  (`/Engine/EditorBlueprintResources/StandardMacros.DoOnce` false :!label _label
    (:`Completed`
      (set `self.IsHit` true)
      (`/Game/Blueprints/Enemy/BP_EnemyCharacter.ExpressKill` _asbp_enemy_character)
      (set `self.Health` (- (`self.Health`) 1.0))
      (if (<= (`self.Health`) 0.0)
        ;[1 1 1] Death
        (`GameplayStatics.PlaySound2D` "/Game/Audio/SoundEffects/Werewolf/Cue_WolfDeath.Cue_WolfDeath" 1.0 1.0 0.0 null null)
        (`KismetSystemLibrary.Delay` 4.0)
        (`GameplayStatics.OpenLevel` "EndingCutscene")
        (else
          (set `/Game/Blueprints/Werewolf/BP_BossTrigger.HasHitWerewolf` true (`self.BossTrigger`))
          (`GameplayStatics.PlaySound2D` "/Game/Audio/SoundEffects/Werewolf/Cue_WerewolfHit.Cue_WerewolfHit" 1.0 1.0 0.0 null null)
          (`KismetSystemLibrary.Delay` 2.0)
          (set `self.IsHit` false)
          (`self.Attack`)
          (goto _label :!via `Reset`))))))

(event `Attack`
  (bind _capsulecomponent (`self.CapsuleComponent`))
  (bind (_returnvalue_roll _returnvalue_pitch) (`KismetMathLibrary.BreakRotator` (`SceneComponent.K2_GetComponentRotation` _capsulecomponent)))
  (bind (_returnvalue_roll_2 _returnvalue_pitch_2 _returnvalue_yaw) (`KismetMathLibrary.BreakRotator` (`KismetMathLibrary.FindLookAtRotation` (`SceneComponent.K2_GetComponentLocation` _capsulecomponent) (`SceneComponent.K2_GetComponentLocation` (`Character.Mesh` (`self.Player`))))))
  ;[1 1 1] Attack Loop
  (`|ExecutionSequence`
    (:`then_0`
      (`SceneComponent.K2_SetWorldRotation` _capsulecomponent (`KismetMathLibrary.MakeRotator` _returnvalue_roll _returnvalue_pitch _returnvalue_yaw) false false :!label _label_2)
      (`KismetSystemLibrary.Delay` 0.2)
      (goto _label_2))
    (:`then_1`
      (if (`self.PlayerVisible`)
        (set `self.IsThrowing` true)
        (if (not (`self.IsHit`))
          (`KismetSystemLibrary.Delay` 2.45)
          (if (not (`self.IsHit`))
            (`GameplayStatics.PlaySound2D` "/Game/Audio/SoundEffects/Werewolf/Cue_Throw.Cue_Throw" 1.0 1.0 0.0 null null)
            (`|SpawnActorFromClass` "/Game/Blueprints/BP_GunProjectile.BP_GunProjectile_C" (`KismetMathLibrary.MakeTransform` (`SceneComponent.K2_GetComponentLocation` (`self.ObjectSpawner`)) (`KismetMathLibrary.MakeRotator` (+ (.roll (`KismetMathLibrary.FindLookAtRotation` (`SceneComponent.K2_GetComponentLocation` (`self.ObjectSpawner`)) (`SceneComponent.K2_GetComponentLocation` (`Character.Mesh` (`self.Player`))))) (`KismetMathLibrary.RandomFloatInRange` -0.5 0.5)) (+ (`KismetMathLibrary.RandomFloatInRange` -0.5 0.5) (.pitch (`KismetMathLibrary.FindLookAtRotation` (`SceneComponent.K2_GetComponentLocation` (`self.ObjectSpawner`)) (`SceneComponent.K2_GetComponentLocation` (`Character.Mesh` (`self.Player`)))))) (+ (`KismetMathLibrary.RandomFloatInRange` -0.5 0.5) (.yaw (`KismetMathLibrary.FindLookAtRotation` (`SceneComponent.K2_GetComponentLocation` (`self.ObjectSpawner`)) (`SceneComponent.K2_GetComponentLocation` (`Character.Mesh` (`self.Player`)))))))) "AdjustIfPossibleButDontSpawnIfColliding" "OverrideRootScale" null 0 (0.0 0.0 0.0) false true null) ; Spawn projectile
            (`KismetSystemLibrary.Delay` 2.43)
            (if (not (`self.IsHit`))
              (`self.Attack`))))
        (else
          (set `self.IsThrowing` false))))))

(fn `UserConstructionScript`)