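; Boss-fight trigger that starts the werewolf encounter once, when the player enters its box.
; The overlap raises the boss elevator, moves the obscuring actors down, then spawns the wolf and first enemy on timed delays, passing itself to both spawners.
; Continue spawns further enemies from a random brigade spawner, indexed up to the array length cached at construction.
; Spawner-removal logic on werewolf hit is disconnected.
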(event `self.ReceiveBeginPlay`
  (set `self.BossTriggerRef` self))

(event `self.Box.OnComponentBeginOverlap`
  (params (OverlappedComponent :type "PrimitiveComponent Object Reference") (OtherActor :type "Actor Object Reference") (OtherComp :type "PrimitiveComponent Object Reference") (OtherBodyIndex :type Integer) (bFromSweep :type Boolean) (SweepResult :type "HitResult Structure (by ref)"))
  (bind _bosstriggerref (`self.BossTriggerRef`))
  (cast `/Game/Blueprints/Player/BP_PlayerCharacter` OtherActor)
  (`/Engine/EditorBlueprintResources/StandardMacros.DoOnce` false
    (:`Completed`
      (`/Game/Blueprints/EnvironmentBPs/WerewolfElevator.RaiseBoss` (`self.ElevatorRef`))
      (`KismetSystemLibrary.Delay` 3.0)
      (for _array_element (`self.Obscure`)
        (`/Game/Blueprints/EnvironmentBPs/WerewolfObscure.MoveDownWObscure` _array_element))
      (`/Game/Blueprints/Werewolf/WerewolfSpawner.SpawnWolf` (`self.WerewolfSpawner`) _bosstriggerref)
      (`KismetSystemLibrary.Delay` 1.0)
      (`/Game/Blueprints/Enemy/BP_EnemySpawner.SpawnEnemy` (`self.FirstEnemy`) _bosstriggerref))))

(event `Continue`
  (`KismetSystemLibrary.Delay` 1.0)
  (`/Game/Blueprints/Enemy/BP_EnemySpawner.SpawnEnemy` (`|GetArrayItem` (`self.BrigadeSpawners`) (`KismetMathLibrary.RandomIntegerInRange` 0 (`self.ArraySize`))) (`self.BossTriggerRef`)))

(fn `UserConstructionScript`
  (set `self.ArraySize` (`KismetArrayLibrary.Array_Length` (`self.BrigadeSpawners`))))