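; BP_TutorialInfo is an actor that displays a tutorial message in the level.
; The construction script fills the Text component from WhatDoesItSay and shows or hides component R based on the Arrow flag.
; At BeginPlay a timeline drives the Mesh's relative Z location, scaling its track value by a fixed amount.
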(event `self.ReceiveBeginPlay`
  (bind (_direction _newtrack_0) (`Timeline|Timeline_0`)
    (:`Update`
      (`SceneComponent.K2_SetRelativeLocation` (`self.Mesh`) (`KismetMathLibrary.MakeVector` 0.0 0.0 (* _newtrack_0 30.0)) false false))))

(fn `UserConstructionScript`
  (`TextRenderComponent.K2_SetText` (`self.Text`) (`self.WhatDoesItSay?`))
  (`SceneComponent.SetVisibility` (`self.r`) (`self.Arrow?`) false))