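; BP_SpaceDebris is an environment actor that animates a piece of space debris with a vertical offset and rotation.
; The construction script applies the Mesh variable to the StaticMesh component, so the displayed mesh is configurable.
; On BeginPlay, two timelines start: one drives the mesh's relative Z location, the other its pitch and yaw together.
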(event `self.ReceiveBeginPlay`
  (bind _staticmesh (`self.StaticMesh`))
  (`|ExecutionSequence`
    (:`then_0`
      (bind (_direction _newtrack_0) (`Timeline|Timeline_0`)
        (:`Update`
          (`SceneComponent.K2_SetRelativeLocation` _staticmesh (`KismetMathLibrary.MakeVector` 0.0 0.0 (* _newtrack_0 30.0)) false false))))
    (:`then_1`
      (bind (_direction_2 _newtrack_0_2) (`Timeline|Timeline_1`)
        (:`Update`
          (bind _returnvalue (* _newtrack_0_2 360.0))
          (`SceneComponent.K2_SetRelativeRotation` _staticmesh (`KismetMathLibrary.MakeRotator` 0.0 _returnvalue _returnvalue) false false))))))

(fn `UserConstructionScript`
  (`StaticMeshComponent.SetStaticMesh` (`self.StaticMesh`) (`self.Mesh`)))