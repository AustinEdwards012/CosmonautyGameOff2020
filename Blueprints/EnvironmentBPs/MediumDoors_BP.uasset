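; Automatic sliding medium door that opens when BP_PlayerCharacter enters its CollisionOpen volume and closes shortly after they leave.
; Two timelines slide the panels along relative Y, each named for the side opposite the mesh it moves, and reverse after a brief delay on exit.
; Each overlap plays a pitched-up hydraulic sound at the actor, using the close-named clip on opening and the open-named clip on closing.
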(event `self.CollisionOpen.OnComponentBeginOverlap`
  (params (OverlappedComponent :type "PrimitiveComponent Object Reference") (OtherActor :type "Actor Object Reference") (OtherComp :type "PrimitiveComponent Object Reference") (OtherBodyIndex :type Integer) (bFromSweep :type Boolean) (SweepResult :type "HitResult Structure (by ref)"))
  (cast `/Game/Blueprints/Player/BP_PlayerCharacter` OtherActor)
  (set `self.IsMidDoorOpen?` true)
  (`|ExecutionSequence`
    (:`then_0`
      (if (`self.IsMidDoorOpen?`)
        (bind (_direction _left_door_slide) (`Timeline|Left_Side_Door_Timeline` :!label _label)
          (:`Update`
            (`SceneComponent.K2_SetRelativeLocation` (`self.RightSideMediumDoor_400x200_LP`) (`KismetMathLibrary.MakeVector` 0.0 _left_door_slide) false false)))))
    (:`then_1`
      (if (`self.IsMidDoorOpen?`)
        (bind (_direction_2 _right_door_slide) (`Timeline|Right_Side_Door_Timeline` :!label _label_2)
          (:`Update`
            (`SceneComponent.K2_SetRelativeLocation` (`self.LeftSideMediumDoor_400x200_LP`) (`KismetMathLibrary.MakeVector` 0.0 _right_door_slide) false false)))))
    (:`then_2`
      (`GameplayStatics.PlaySoundAtLocation` "/Game/Audio/SoundEffects/Environment/sfx_hydraulic_door_close.sfx_hydraulic_door_close" (`self.K2_GetActorLocation`) (struct) 1.0 1.5 0.0 "/Game/Audio/SoundEffects/GameAttenuation.GameAttenuation" "/Game/Audio/SoundEffects/GameConcurrency.GameConcurrency" null))))

(event `self.CollisionOpen.OnComponentEndOverlap`
  (params (OverlappedComponent :type "PrimitiveComponent Object Reference") (OtherActor :type "Actor Object Reference") (OtherComp :type "PrimitiveComponent Object Reference") (OtherBodyIndex :type Integer))
  (cast `/Game/Blueprints/Player/BP_PlayerCharacter` OtherActor)
  (set `self.IsMidDoorOpen?` false)
  (`|ExecutionSequence`
    (:`then_0`
      (if (not (`self.IsMidDoorOpen?`))
        (`KismetSystemLibrary.Delay` 0.2)
        (goto _label :!via `Reverse`)))
    (:`then_1`
      (if (not (`self.IsMidDoorOpen?`))
        (`KismetSystemLibrary.Delay` 0.2)
        (goto _label_2 :!via `Reverse`)))
    (:`then_2`
      (`GameplayStatics.PlaySoundAtLocation` "/Game/Audio/SoundEffects/Environment/sfx_hydraulic_door_open.sfx_hydraulic_door_open" (`self.K2_GetActorLocation`) (struct) 1.0 1.5 0.0 "/Game/Audio/SoundEffects/GameAttenuation.GameAttenuation" "/Game/Audio/SoundEffects/GameConcurrency.GameConcurrency" null))))

(fn `UserConstructionScript`)