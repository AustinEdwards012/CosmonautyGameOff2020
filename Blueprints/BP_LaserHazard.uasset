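; BP_LaserHazard is a laser hazard actor that kills the player on hit.
; The Hit event casts the other actor to BP_PlayerCharacter, sets its PlayerHealth to zero and calls RegisterHit.
; The construction script uses the Goal flag to swap visibility between two scene hierarchies and disable Box collision, making goal variants non-colliding.
; A MinusOneEndBar flag hides one particle system.
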(event `self.ReceiveHit`
  (params (MyComp :type "PrimitiveComponent Object Reference") (Other :type "Actor Object Reference") (OtherComp :type "PrimitiveComponent Object Reference") (bSelfMoved :type Boolean) (HitLocation :type "Vector Structure") (HitNormal :type "Vector Structure") (NormalImpulse :type "Vector Structure") (Hit :type "HitResult Structure (by ref)"))
  (`/Engine/EditorBlueprintResources/StandardMacros.IsValid` Other
    (:`Is Valid`
      (bind _asbp_player_character (cast `/Game/Blueprints/Player/BP_PlayerCharacter` Other))
      (set `/Game/Blueprints/Player/BP_PlayerCharacter.PlayerHealth` 0.0 _asbp_player_character)
      (`/Game/Blueprints/Player/BP_PlayerCharacter.RegisterHit` _asbp_player_character))))

(fn `UserConstructionScript`
  (bind _goal_ (`self.Goal?`))
  (bind _box (`self.Box`))
  (`SceneComponent.SetVisibility` (`self.Scene1`) _goal_ true)
  (`SceneComponent.SetVisibility` (`self.Scene`) (not _goal_) true)
  (`SceneComponent.SetVisibility` (`self.ParticleSystem3`) (not (`self.MinusOneEndBar`)) false)
  (if _goal_
    (`PrimitiveComponent.SetCollisionEnabled` _box "NoCollision")
    (else
      (`PrimitiveComponent.SetCollisionEnabled` _box "QueryAndPhysics"))))