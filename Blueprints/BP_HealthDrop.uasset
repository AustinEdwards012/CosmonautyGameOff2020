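; Timed health pickup that restores a fixed amount of PlayerHealth, up to a cap, when BP_PlayerCharacter overlaps its sphere.
; On BeginPlay, SpawnEffect drives a dynamic material's Invisible and Energy parameters through chained timelines, then swaps to the ready material.
; Despawn then waits briefly, restores the transfer material, animates Energy then Invisible, and destroys the actor.
; Pickup fires once, playing sound and particles before destroying it.
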(event `self.ReceiveBeginPlay`
  (bind _pickupmat (`self.PickupMat`))
  (bind _pickupmat_2 (`self.PickupMat`))
  (`GameplayStatics.SpawnEmitterAtLocation` "/Game/Particles/Enemies/P_Spawn.P_Spawn" (`self.K2_GetActorLocation`))
  (bind (_direction _spawnin) (`Timeline|Timeline_0` :!via `PlayFromStart`)
    (:`Update`
      (set `self.Invisible` _spawnin)
      (`MaterialInstanceDynamic.SetScalarParameterValue` _pickupmat "Invisible" (`self.Invisible`) :!label _label)
      (`MaterialInstanceDynamic.SetScalarParameterValue` _pickupmat "Energy" (`self.Energy`)))
    (:`Finished`
      (`GameplayStatics.PlaySoundAtLocation` "/Game/Audio/SoundEffects/Cosmonaut/Cue_Spawn.Cue_Spawn" (`self.K2_GetActorLocation`) (struct) 1.0 1.0 0.0 "/Game/Audio/SoundEffects/GameAttenuation.GameAttenuation" "/Game/Audio/SoundEffects/GameConcurrency.GameConcurrency" null)
      (bind (_direction_2 _spawnin_2) (`Timeline|Timeline_1` :!via `PlayFromStart`)
        (:`Update`
          (set `self.Energy` _spawnin_2)
          (goto _label))
        (:`Finished`
          (`PrimitiveComponent.SetMaterial` (`self.HealthDropMesh`) 0 "/Game/Materials/Mat_HealthPickup_Ready.Mat_HealthPickup_Ready")
          (`KismetSystemLibrary.Delay` 3.0)
          (bind _returnvalue (`PrimitiveComponent.CreateDynamicMaterialInstance` (`self.HealthDropMesh`) 0 "/Game/Materials/Mat_HealthPickup_Transfer.Mat_HealthPickup_Transfer" "None"))
          (bind _output_get (set `self.PickupMat` _returnvalue))
          (`MaterialInstanceDynamic.SetScalarParameterValue` _output_get "Invisible" (`self.Invisible`))
          (`MaterialInstanceDynamic.SetScalarParameterValue` _output_get "Energy" (`self.Energy`))
          (`GameplayStatics.PlaySoundAtLocation` "/Game/Audio/SoundEffects/Cosmonaut/Cue_Spawn.Cue_Spawn" (`self.K2_GetActorLocation`) (struct) 1.0 1.0 0.0 "/Game/Audio/SoundEffects/GameAttenuation.GameAttenuation" "/Game/Audio/SoundEffects/GameConcurrency.GameConcurrency" null)
          (bind (_direction_3 _spawnin_3) (`Timeline|Timeline_3` :!via `PlayFromStart`)
            (:`Update`
              (set `self.Energy` _spawnin_3)
              (`MaterialInstanceDynamic.SetScalarParameterValue` _pickupmat_2 "Invisible" (`self.Invisible`) :!label _label_2)
              (`MaterialInstanceDynamic.SetScalarParameterValue` _pickupmat_2 "Energy" (`self.Energy`)))
            (:`Finished`
              (bind (_direction_4 _spawnin_4) (`Timeline|Timeline_2` :!via `PlayFromStart`)
                (:`Update`
                  (set `self.Invisible` _spawnin_4)
                  (goto _label_2))
                (:`Finished`
                  (`self.K2_DestroyActor`))))))))))

(event `self.Sphere.OnComponentBeginOverlap`
  (params (OverlappedComponent :type "PrimitiveComponent Object Reference") (OtherActor :type "Actor Object Reference") (OtherComp :type "PrimitiveComponent Object Reference") (OtherBodyIndex :type Integer) (bFromSweep :type Boolean) (SweepResult :type "HitResult Structure (by ref)"))
  (bind _asbp_player_character (cast `/Game/Blueprints/Player/BP_PlayerCharacter` OtherActor))
  (`/Engine/EditorBlueprintResources/StandardMacros.DoOnce` false
    (:`Completed`
      (`GameplayStatics.PlaySoundAtLocation` "/Game/Audio/SoundEffects/Environment/sfx_health_pack.sfx_health_pack" (`self.K2_GetActorLocation`) (struct) 1.0 1.0 0.0 "/Game/Audio/SoundEffects/GameAttenuation.GameAttenuation" "/Game/Audio/SoundEffects/GameConcurrency.GameConcurrency" null)
      (`GameplayStatics.SpawnEmitterAtLocation` "/Game/Particles/Enemies/P_Spawn.P_Spawn" (`self.K2_GetActorLocation`))
      (bind _playerhealth (`/Game/Blueprints/Player/BP_PlayerCharacter.PlayerHealth` _asbp_player_character))
      (set `/Game/Blueprints/Player/BP_PlayerCharacter.PlayerHealth` (+ _playerhealth 3.0) _asbp_player_character)
      (if (> _playerhealth 10.0)
        (set `/Game/Blueprints/Player/BP_PlayerCharacter.PlayerHealth` 10.0 _asbp_player_character))
      (`self.K2_DestroyActor`))))

(fn `UserConstructionScript`
  (bind _returnvalue (`PrimitiveComponent.CreateDynamicMaterialInstance` (`self.HealthDropMesh`) 0 "/Game/Materials/Mat_HealthPickup_Transfer.Mat_HealthPickup_Transfer" "None"))
  (bind _output_get (set `self.PickupMat` _returnvalue))
  (`MaterialInstanceDynamic.SetScalarParameterValue` _output_get "Invisible" (`self.Invisible`))
  (`MaterialInstanceDynamic.SetScalarParameterValue` _output_get "Energy" (`self.Energy`)))