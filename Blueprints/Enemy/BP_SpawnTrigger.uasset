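; BP_SpawnTrigger is a level trigger volume that spawns and/or kills enemies when the player first overlaps its box.
; With Kill on, it kills every BP_EnemyCharacter whose SpawnerNumber matches NumberToKill.
; With Spawn on, it sets NumberToSpawn as the SpawnerNumber on each connected spawner and tells it to spawn an enemy, each action firing once.
; The construction script swaps the billboard icon to show the configured Spawn/Kill mode.
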(event `self.Box.OnComponentBeginOverlap`
  (params (OverlappedComponent :type "PrimitiveComponent Object Reference") (OtherActor :type "Actor Object Reference") (OtherComp :type "PrimitiveComponent Object Reference") (OtherBodyIndex :type Integer) (bFromSweep :type Boolean) (SweepResult :type "HitResult Structure (by ref)"))
  (cast `/Game/Blueprints/Player/BP_PlayerCharacter` OtherActor)
  (if (`self.Kill?`)
    (`/Engine/EditorBlueprintResources/StandardMacros.DoOnce` false
      (:`Completed`
        (bind _outactors (`GameplayStatics.GetAllActorsOfClass` "/Game/Blueprints/Enemy/BP_EnemyCharacter.BP_EnemyCharacter_C"))
        (for _array_element _outactors
          (if (== (`/Game/Blueprints/Enemy/BP_EnemyCharacter.SpawnerNumber` _array_element) (`self.NumberToKill`))
            (`/Game/Blueprints/Enemy/BP_EnemyCharacter.Kill` _array_element))))))
  (if (`self.Spawn?`)
    (`/Engine/EditorBlueprintResources/StandardMacros.DoOnce` false
      (:`Completed`
        (for _array_element_2 (`self.ConnectedSpawners`)
          (set `/Game/Blueprints/Enemy/BP_EnemySpawner.SpawnerNumber` (`self.NumberToSpawn`) _array_element_2)
          (`/Game/Blueprints/Enemy/BP_EnemySpawner.SpawnEnemy` _array_element_2 null))))))

(fn `UserConstructionScript`
  (if (and (`self.Spawn?`) (`self.Kill?`))
    (`BillboardComponent.SetSprite` (`self.Billboard`) "/Game/PrototypingStuff/SpawnKillIcon.SpawnKillIcon")
    (elif (`self.Spawn?`)
      (`BillboardComponent.SetSprite` (`self.Billboard`) "/Game/PrototypingStuff/SpawnIcon.SpawnIcon")
      (elif (`self.Kill?`)
        (`BillboardComponent.SetSprite` (`self.Billboard`) "/Game/PrototypingStuff/KillIcon.KillIcon")
        (else
          (`BillboardComponent.SetSprite` (`self.Billboard`) "/Game/PrototypingStuff/SpawnerUnset.SpawnerUnset"))))))