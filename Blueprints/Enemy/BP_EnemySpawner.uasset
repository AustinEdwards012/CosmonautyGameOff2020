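; BP_EnemySpawner is a placeable spawner that creates a BP_EnemyCharacter when its SpawnEnemy event is called with a boss trigger reference.
; It spawns slightly above itself, passing along enemy type, jetpack, active state, search radius, spawner number, respawn point and arrow-based facing, then clears the enemy's AIControllerClass.
; The construction script previews those settings through a type-colored billboard icon, movement and activity labels, and an optional search-radius sphere.
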(event `SpawnEnemy`
  (params (BossTriggerReference :type "/Game/Blueprints/Werewolf/BP_BossTrigger Object Reference"))
  (bind (_returnvalue_x _returnvalue_y _returnvalue_z) (`KismetMathLibrary.BreakVector` (`self.K2_GetActorLocation`)))
  (bind (_returnvalue_roll _returnvalue_pitch _returnvalue_yaw) (`KismetMathLibrary.BreakRotator` (`SceneComponent.K2_GetComponentRotation` (`self.Arrow`))))
  (bind _returnvalue (`KismetMathLibrary.MakeVector` _returnvalue_x _returnvalue_y (+ _returnvalue_z 80.0)))
  (bind _returnvalue_2 (`|SpawnActorFromClass` "/Game/Blueprints/Enemy/BP_EnemyCharacter.BP_EnemyCharacter_C" (`KismetMathLibrary.MakeTransform` _returnvalue) "Undefined" "OverrideRootScale" null (`self.ActiveCosmonaut`) (`self.HasJetpack`) _returnvalue false (`self.SpawnerNumber`) _returnvalue_yaw (`self.SetSearchRadius`) (`self.Fodder?`) (`self.Wolf?`) BossTriggerReference null))
  (set `Pawn.AIControllerClass` null _returnvalue_2))

(fn `UserConstructionScript`
  (bind _movementtype (`self.MovementType`))
  (bind _alertradiusdisplay (`self.AlertRadiusDisplay`))
  (if (`self.Wolf?`)
    (`BillboardComponent.SetSprite` (`self.Billboard`) "/Game/Other/SpawnerIconRed.SpawnerIconRed")
    (elif (`self.Fodder?`)
      (`BillboardComponent.SetSprite` (`self.Billboard`) "/Game/Other/SpawnerIconBlue.SpawnerIconBlue")
      (else
        (`BillboardComponent.SetSprite` (`self.Billboard`) "/Game/Other/SpawnerIconOrange.SpawnerIconOrange"))))
  (`SceneComponent.SetVisibility` _alertradiusdisplay (`self.ShowAlertEscapeRadius`) false)
  (`SphereComponent.SetSphereRadius` _alertradiusdisplay (`self.SetSearchRadius`) true)
  (if (`self.HasJetpack`)
    (`TextRenderComponent.K2_SetText` _movementtype (`KismetTextLibrary.Conv_StringToText` "Jetpack"))
    (`TextRenderComponent.K2_SetText` (`self.ActiveType`) (`KismetTextLibrary.Conv_StringToText` "N/A"))
    (else
      (`TextRenderComponent.K2_SetText` _movementtype (`KismetTextLibrary.Conv_StringToText` "Ground"))
      (if (`self.ActiveCosmonaut`)
        (`TextRenderComponent.K2_SetText` (`self.ActiveType`) (`KismetTextLibrary.Conv_StringToText` "Active"))
        (else
          (`TextRenderComponent.K2_SetText` (`self.ActiveType`) (`KismetTextLibrary.Conv_StringToText` "Inactive")))))))